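; WaterSourceBlueprint is a water source actor that sprays fire-extinguishing WaterProjectileBlueprint projectiles while IsWaterComing is true.
; Tick counts SpawnTimer down, spawns a projectile at the actor's transform when it expires, then restores the interval from the class default.
; Each projectile's static mesh receives a random physics velocity within a narrow cone around the Sphere component's up vector.
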(event `self.ReceiveBeginPlay`
  (set `self.SpawnTimer` 0.0))

(event `self.ReceiveTick`
  (params (DeltaSeconds :type "Float (single-precision)"))
  (bind _output_get (set `self.SpawnTimer` (- (`self.SpawnTimer`) DeltaSeconds)))
  (if (and (`self.IsWaterComing`) (<= _output_get 0.0))
    (`|ExecutionSequence`
      (:`then_0`
        (set `self.SpawnTimer` (defaults `/Game/Blueprints/WaterSourceBlueprint` "WaterSourceBlueprint_C")))
      (:`then_1`
        (bind _returnvalue (`|SpawnActorFromClass` "/Game/Blueprints/WaterProjectileBlueprint.WaterProjectileBlueprint_C" (`self.GetTransform` self) "Undefined" "OverrideRootScale" null null))
        (`PrimitiveComponent.SetPhysicsLinearVelocity` (`self.GetComponentByClass` _returnvalue "/Script/Engine.StaticMeshComponent") (* (`KismetMathLibrary.RandomUnitVectorInConeInDegrees` (`SceneComponent.GetUpVector` (`self.Sphere`)) 20.0) (`KismetMathLibrary.Conv_DoubleToVector` (`KismetMathLibrary.RandomFloatInRange` 800.0 1000.0))) false "None")))))

(fn `NewFunction_0`
  (params (NewParam :type "NiagaraParticleCallbackHandler Interface")))

(fn `UserConstructionScript`)